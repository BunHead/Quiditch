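; Goals actor that detects projectiles passing through two teams' goals and keeps each team's score.
; Each goal has left, middle and right trigger pairs; entering a back or front trigger sets or clears one shared CorrectDirection flag.
; Leaving a back trigger with the flag set starts a retriggerable delay, then increments that team's score and calls Goal on MyProjectile.
; Both teams' debug messages print "Team 2 Goal".
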(event OnComponentBeginOverlap(Team2RightBack)
  (params (OtherActor :type Actor%20Object%20Reference) (OtherComp :type Primitive%20Component%20Object%20Reference) (OtherBodyIndex :type Integer) (bFromSweep :type Boolean) (SweepResult :type Hit%20Result%20Structure%20%28by%20ref%29))
  ;[1 1 1] Set Direction Check
  (Variables|Default|SetCorrectDirection true))

(event OnComponentBeginOverlap(Team2RightFront)
  (params (OtherActor :type Actor%20Object%20Reference) (OtherComp :type Primitive%20Component%20Object%20Reference) (OtherBodyIndex :type Integer) (bFromSweep :type Boolean) (SweepResult :type Hit%20Result%20Structure%20%28by%20ref%29))
  ;[1 1 1] Set Direction Check
  (Variables|Default|SetCorrectDirection false))

(event OnComponentBeginOverlap(Team2LeftFront)
  (params (OtherActor :type Actor%20Object%20Reference) (OtherComp :type Primitive%20Component%20Object%20Reference) (OtherBodyIndex :type Integer) (bFromSweep :type Boolean) (SweepResult :type Hit%20Result%20Structure%20%28by%20ref%29))
  ;[1 1 1] Set Direction Check
  (Variables|Default|SetCorrectDirection false))

(event OnComponentBeginOverlap(Team2LeftBack)
  (params (OtherActor :type Actor%20Object%20Reference) (OtherComp :type Primitive%20Component%20Object%20Reference) (OtherBodyIndex :type Integer) (bFromSweep :type Boolean) (SweepResult :type Hit%20Result%20Structure%20%28by%20ref%29))
  ;[1 1 1] Set Direction Check
  (Variables|Default|SetCorrectDirection true))

(event OnComponentEndOverlap(Team2LeftBack)
  (params (OtherActor :type Actor%20Object%20Reference) (OtherComp :type Primitive%20Component%20Object%20Reference) (OtherBodyIndex :type Integer))
  ;[1 1 1] Team2
  (Variables|Default|SetProjectile OtherActor)
  (if (Variables|Default|GetCorrectDirection)
    (Utilities|FlowControl|RetriggerableDelay 3.0)
    (bind _output_get (Variables|Default|SetTeam2Score (+ (Variables|Default|GetTeam2Score) 1)))
    (Development|PrintString (Utilities|String|ToString(Text) (Utilities|Text|FormatText "Team 2 Goal: {Score}" (Utilities|Text|ToText(Integer) _output_get))))
    (CallFunction|GOAL (Variables|Default|GetProjectile))))

(event OnComponentEndOverlap(Team2RightBack)
  (params (OtherActor :type Actor%20Object%20Reference) (OtherComp :type Primitive%20Component%20Object%20Reference) (OtherBodyIndex :type Integer))
  ;[1 1 1] Team2
  (Variables|Default|SetProjectile OtherActor)
  (if (Variables|Default|GetCorrectDirection)
    (Utilities|FlowControl|RetriggerableDelay 3.0)
    (bind _output_get (Variables|Default|SetTeam2Score (+ (Variables|Default|GetTeam2Score) 1)))
    (Development|PrintString (Utilities|String|ToString(Text) (Utilities|Text|FormatText "Team 2 Goal: {Score}" (Utilities|Text|ToText(Integer) _output_get))))
    (CallFunction|GOAL (Variables|Default|GetProjectile))))

(event OnComponentBeginOverlap(Team2MiddleFront)
  (params (OtherActor :type Actor%20Object%20Reference) (OtherComp :type Primitive%20Component%20Object%20Reference) (OtherBodyIndex :type Integer) (bFromSweep :type Boolean) (SweepResult :type Hit%20Result%20Structure%20%28by%20ref%29))
  ;[1 1 1] Set Direction Check
  (Variables|Default|SetCorrectDirection false))

(event OnComponentBeginOverlap(Team2MiddleBack)
  (params (OtherActor :type Actor%20Object%20Reference) (OtherComp :type Primitive%20Component%20Object%20Reference) (OtherBodyIndex :type Integer) (bFromSweep :type Boolean) (SweepResult :type Hit%20Result%20Structure%20%28by%20ref%29))
  ;[1 1 1] Set Direction Check
  (Variables|Default|SetCorrectDirection true))

(event OnComponentEndOverlap(Team2MiddleBack)
  (params (OtherActor :type Actor%20Object%20Reference) (OtherComp :type Primitive%20Component%20Object%20Reference) (OtherBodyIndex :type Integer))
  ;[1 1 1] Team2
  (Variables|Default|SetProjectile OtherActor)
  (if (Variables|Default|GetCorrectDirection)
    (Utilities|FlowControl|RetriggerableDelay 3.0)
    (bind _output_get (Variables|Default|SetTeam2Score (+ (Variables|Default|GetTeam2Score) 1)))
    (Development|PrintString (Utilities|String|ToString(Text) (Utilities|Text|FormatText "Team 2 Goal: {Score}" (Utilities|Text|ToText(Integer) _output_get))))
    (CallFunction|GOAL (Variables|Default|GetProjectile))))

(event OnComponentBeginOverlap(Team1LeftFront)
  (params (OtherActor :type Actor%20Object%20Reference) (OtherComp :type Primitive%20Component%20Object%20Reference) (OtherBodyIndex :type Integer) (bFromSweep :type Boolean) (SweepResult :type Hit%20Result%20Structure%20%28by%20ref%29))
  ;[1 1 1] Set Direction Check
  (Variables|Default|SetCorrectDirection false))

(event OnComponentBeginOverlap(Team1RightFront)
  (params (OtherActor :type Actor%20Object%20Reference) (OtherComp :type Primitive%20Component%20Object%20Reference) (OtherBodyIndex :type Integer) (bFromSweep :type Boolean) (SweepResult :type Hit%20Result%20Structure%20%28by%20ref%29))
  ;[1 1 1] Set Direction Check
  (Variables|Default|SetCorrectDirection false))

(event OnComponentBeginOverlap(Team1MiddleFront)
  (params (OtherActor :type Actor%20Object%20Reference) (OtherComp :type Primitive%20Component%20Object%20Reference) (OtherBodyIndex :type Integer) (bFromSweep :type Boolean) (SweepResult :type Hit%20Result%20Structure%20%28by%20ref%29))
  ;[1 1 1] Set Direction Check
  (Variables|Default|SetCorrectDirection false))

(event OnComponentBeginOverlap(Team1RightBack)
  (params (OtherActor :type Actor%20Object%20Reference) (OtherComp :type Primitive%20Component%20Object%20Reference) (OtherBodyIndex :type Integer) (bFromSweep :type Boolean) (SweepResult :type Hit%20Result%20Structure%20%28by%20ref%29))
  ;[1 1 1] Set Direction Check
  (Variables|Default|SetCorrectDirection true))

(event OnComponentBeginOverlap(Team1MiddleBack)
  (params (OtherActor :type Actor%20Object%20Reference) (OtherComp :type Primitive%20Component%20Object%20Reference) (OtherBodyIndex :type Integer) (bFromSweep :type Boolean) (SweepResult :type Hit%20Result%20Structure%20%28by%20ref%29))
  ;[1 1 1] Set Direction Check
  (Variables|Default|SetCorrectDirection true))

(event OnComponentBeginOverlap(Team1LeftBack)
  (params (OtherActor :type Actor%20Object%20Reference) (OtherComp :type Primitive%20Component%20Object%20Reference) (OtherBodyIndex :type Integer) (bFromSweep :type Boolean) (SweepResult :type Hit%20Result%20Structure%20%28by%20ref%29))
  ;[1 1 1] Set Direction Check
  (Variables|Default|SetCorrectDirection true))

(event OnComponentEndOverlap(Team1RightBack)
  (params (OtherActor :type Actor%20Object%20Reference) (OtherComp :type Primitive%20Component%20Object%20Reference) (OtherBodyIndex :type Integer))
  ;[1 1 1] Team 1
  (Variables|Default|SetProjectile OtherActor)
  (if (Variables|Default|GetCorrectDirection)
    (Utilities|FlowControl|RetriggerableDelay 3.0)
    (bind _output_get (Variables|Default|SetTeam1Score (+ (Variables|Default|GetTeam1Score) 1)))
    (Development|PrintString (Utilities|String|ToString(Text) (Utilities|Text|FormatText "Team 2 Goal: {Score}" (Utilities|Text|ToText(Integer) _output_get))))
    (CallFunction|GOAL (Variables|Default|GetProjectile))))

(event OnComponentEndOverlap(Team1MiddleBack)
  (params (OtherActor :type Actor%20Object%20Reference) (OtherComp :type Primitive%20Component%20Object%20Reference) (OtherBodyIndex :type Integer))
  ;[1 1 1] Team 1
  (Variables|Default|SetProjectile OtherActor)
  (if (Variables|Default|GetCorrectDirection)
    (Utilities|FlowControl|RetriggerableDelay 3.0)
    (bind _output_get (Variables|Default|SetTeam1Score (+ (Variables|Default|GetTeam1Score) 1)))
    (Development|PrintString (Utilities|String|ToString(Text) (Utilities|Text|FormatText "Team 2 Goal: {Score}" (Utilities|Text|ToText(Integer) _output_get))))
    (CallFunction|GOAL (Variables|Default|GetProjectile))))

(event OnComponentEndOverlap(Team1LeftBack)
  (params (OtherActor :type Actor%20Object%20Reference) (OtherComp :type Primitive%20Component%20Object%20Reference) (OtherBodyIndex :type Integer))
  ;[1 1 1] Team 1
  (Variables|Default|SetProjectile OtherActor)
  (if (Variables|Default|GetCorrectDirection)
    (Utilities|FlowControl|RetriggerableDelay 3.0)
    (bind _output_get (Variables|Default|SetTeam1Score (+ (Variables|Default|GetTeam1Score) 1)))
    (Development|PrintString (Utilities|String|ToString(Text) (Utilities|Text|FormatText "Team 2 Goal: {Score}" (Utilities|Text|ToText(Integer) _output_get))))
    (CallFunction|GOAL (Variables|Default|GetProjectile))))

(event Custom|GOAL
  (params (Projectile :type Actor%20Object%20Reference))
  ;[1 1 1] Cast
  (bind _asmy_projectile (Utilities|Casting|CastToMyProjectile Projectile)
    (:then
      (Default|Goal _asmy_projectile))
    (:CastFailed
      (Development|PrintString "Oh Dear"))))

(event EventBeginPlay)

(event EventActorBeginOverlap
  (params (OtherActor :type Actor%20Object%20Reference)))

(event EventTick
  (params (DeltaSeconds :type Float%20%28single-precision%29)))

(fn ConstructionScript)