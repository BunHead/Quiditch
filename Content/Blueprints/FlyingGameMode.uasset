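; Game mode for a flying game that assigns player starts and handles VR headset recentering.
; The Choose Player Start function returns the first PlayerStart not tagged "Taken" and tags it so later players get another.
; BeginPlay spawns a MyProjectile at a fixed transform with an enormous initial speed, then recenters the headset if VR is enabled or prints a warning otherwise.
; Space bar triggers the same orientation and position reset.
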(event EventBeginPlay
  ;[1 1 1] Detect VR
  (Utilities|FlowControl|Sequence
    (:then_0
      (Game|SpawnActorfromClass "/Game/Blueprints/MyProjectile.MyProjectile_C" (Math|Transform|MakeTransform "-2000.000000,-27000.000000,4500.000000" "10.000000,150.000000,0.000000") "AlwaysSpawn" 0 1e+15 0))
    (:then_1
      (if (Class|HeadMountedDisplayFunctionLibrary|IsHeadMountedDisplayEnabled)
        (Class|HeadMountedDisplayFunctionLibrary|ResetOrientationandPosition 0.0 "OrientationAndPosition")
        (else
          (Development|PrintString "No VR Detected"))))))

(event Input|KeyboardEvents|SpaceBar
  (params (Key :type Key%20Structure :default "AnyKey"))
  ;[1 1 1] Detect VR
  (:Pressed
    (Class|HeadMountedDisplayFunctionLibrary|ResetOrientationandPosition 0.0 "OrientationAndPosition")))

(fn ConstructionScript)

(fn ChoosePlayerStart
  (bind _outactors (Actor|GetAllActorsOfClass "/Script/Engine.PlayerStart"))
  (bind _array_element (Utilities|Array|ForEachLoopwithBreak _outactors)
    (:LoopBody
      (if (Utilities|Name|NotEqual(Name) (Variables|/Script/Engine.PlayerStart|GetPlayerStartTag _array_element) "Taken")
        (Variables|/Script/Engine.PlayerStart|SetPlayerStartTag _array_element "Taken")
        (Development|PrintText (Utilities|Text|FormatText "Start Position {position}" (Utilities|Text|ToText(Name) (Variables|/Script/Engine.PlayerStart|GetPlayerStartTag _array_element))))
        (return _array_element true)))))