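; QuiditchHUD is a HUD that opens the MainMenu widget for a VRPlayerController.
; It does so on BeginPlay without an enabled headset, or whenever Left Shift, Escape or P is pressed, adding a new instance each time.
; An unused DrawButton helper draws a centred texture and hit box, but its text position ignores the button location and its DrawText receives no string.
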(event EventBeginPlay
  (if (not (Class|HeadMountedDisplayFunctionLibrary|IsHeadMountedDisplayEnabled))
    (bind _asvrplayer_controller (Utilities|Casting|CastToVRPlayerController (Game|Player|GetOwningPlayerController)))
    (bind _returnvalue (UserInterface|CreateWidget "/Game/Menu/MainMenu.MainMenu_C" _asvrplayer_controller))
    (UserInterface|Viewport|AddtoViewport _returnvalue 0)))

(event Input|KeyboardEvents|Escape
  (params (Key :type Key%20Structure :default "AnyKey"))
  (:Pressed
    (bind _asvrplayer_controller (Utilities|Casting|CastToVRPlayerController (Game|Player|GetOwningPlayerController)))
    (bind _returnvalue (UserInterface|CreateWidget "/Game/Menu/MainMenu.MainMenu_C" _asvrplayer_controller))
    (UserInterface|Viewport|AddtoViewport _returnvalue 0)))

(event Input|KeyboardEvents|P
  (params (Key :type Key%20Structure :default "AnyKey"))
  (:Pressed
    (bind _asvrplayer_controller (Utilities|Casting|CastToVRPlayerController (Game|Player|GetOwningPlayerController)))
    (bind _returnvalue (UserInterface|CreateWidget "/Game/Menu/MainMenu.MainMenu_C" _asvrplayer_controller))
    (UserInterface|Viewport|AddtoViewport _returnvalue 0)))

(event Input|KeyboardEvents|LeftShift
  (params (Key :type Key%20Structure :default "AnyKey"))
  (:Pressed
    (bind _asvrplayer_controller (Utilities|Casting|CastToVRPlayerController (Game|Player|GetOwningPlayerController)))
    (bind _returnvalue (UserInterface|CreateWidget "/Game/Menu/MainMenu.MainMenu_C" _asvrplayer_controller))
    (UserInterface|Viewport|AddtoViewport _returnvalue 0)))

(fn ConstructionScript)

(fn DrawButton
  (params (ButtonText :type Text) (ButtonName :type Name :default "None") (ButtonTexture :type Texture%20Object%20Reference) (ButtonScreenLocation :type Vector%202D%20Structure))
  (bind _returnvalue (Math|Vector2D|MakeVector2D 128.0 64.0))
  (bind _returnvalue_2 (Utilities|String|ToString(Text) ButtonText))
  (bind _returnvalue_3 (- ButtonScreenLocation _returnvalue))
  (bind (_outwidth _outheight) (Class|HUD|GetTextSize _returnvalue_2 0 1.5))
  (bind (_x _y) (Math|Vector2D|BreakVector2D _returnvalue_3))
  (bind _returnvalue_4 (Math|Vector2D|MakeVector2D _outwidth _outheight))
  (bind _returnvalue_5 (/ _returnvalue_4 2.0))
  (bind (_x_2 _y_2) (Math|Vector2D|BreakVector2D _returnvalue_5))
  (Class|HUD|DrawTextureSimple ButtonTexture _x _y 1.0 false)
  (HUD|DrawText "" "(R=0,G=0,B=0,A=1)" _x_2 _y_2 0 1.0 false)
  (Class|HUD|AddHitBox _returnvalue_3 (Math|Vector2D|MakeVector2D 256.0 128.0) "None" false))